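; BP_DronePath is a spline path Blueprint, named for drones, that exposes its spline and world-space start location to other objects.
; The construction script tints the spline's segments and tangents with PathColor and enables debug drawing.
; BeginPlay turns that debug drawing off, so the colored path display does not persist into gameplay.
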(event `self.ReceiveBeginPlay`
  (`SplineComponent.SetDrawDebug` (`self.PathSpline`) false))

(fn `Get Path Start Location`
  (returns (StartLoc :type "Vector Structure"))
  (return (`SplineComponent.GetLocationAtSplinePoint` (`self.PathSpline`) 0 "World")))

(fn `GetPathSpline`
  (returns (`Spline Componenet Reference` :type "SplineComponent Object Reference"))
  (return (`self.PathSpline`)))

(fn `UserConstructionScript`
  (bind _pathcolor (`self.PathColor`))
  (bind _pathspline (`self.PathSpline`))
  ;[1 1 1] Color
  (`SplineComponent.SetUnselectedSplineSegmentColor` _pathspline _pathcolor)
  (`SplineComponent.SetSelectedSplineSegmentColor` _pathspline _pathcolor)
  (`SplineComponent.SetTangentColor` _pathspline _pathcolor)
  (`SplineComponent.SetDrawDebug` (`self.PathSpline`) true))