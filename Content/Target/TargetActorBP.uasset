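; Target actor that patrols a looping list of points and prints a hit message when another actor overlaps it.
; Each Tick moves it toward the current point by up to MaxSpeed without sweeping or delta-time scaling, landing exactly when close enough.
; Within AcceptanceRadius it advances the point index, resetting at the array's end.
; Otherwise it calls a Delay that has nothing wired after it.
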(event `self.ReceiveTick`
  (params (DeltaSeconds :type "Float (single-precision)"))
  (bind _returnvalue (`self.K2_GetActorLocation`))
  (bind _maxspeed (`self.MaxSpeed`))
  (bind _returnvalue_2 (- (`|GetArrayItem` (`self.PatrolPoints`) (`self.NextPointIndex`)) _returnvalue))
  (bind _returnvalue_3 (`KismetMathLibrary.VSize` _returnvalue_2))
  (if (<= _returnvalue_3 (`self.MaxSpeed`))
    (`self.K2_SetActorLocation` (+ _returnvalue _returnvalue_2))
    (else
      (`self.K2_SetActorLocation` (+ _returnvalue (* (/ _returnvalue_2 (`KismetMathLibrary.MakeVector` _returnvalue_3 _returnvalue_3 _returnvalue_3)) (`KismetMathLibrary.MakeVector` _maxspeed _maxspeed _maxspeed))))))
  (if (<= (`KismetMathLibrary.VSize` (- (`|GetArrayItem` (`self.PatrolPoints`) (`self.NextPointIndex`)) (`self.K2_GetActorLocation`))) (`self.AcceptanceRadius`))
    (bind _result (`/Engine/EditorBlueprintResources/StandardMacros.IncrementInt` (`self.NextPointIndex`))
      (:`  `
        (if (== _result (`KismetArrayLibrary.Array_Length` (`self.PatrolPoints`)))
          (set `self.NextPointIndex` 0))))
    (else
      (`KismetSystemLibrary.Delay` (`self.MovementDelaySec`)))))

(event `self.ReceiveActorBeginOverlap`
  (params (OtherActor :type "Actor Object Reference"))
  (`KismetSystemLibrary.PrintString` "Hit!"))

(fn `UserConstructionScript`)