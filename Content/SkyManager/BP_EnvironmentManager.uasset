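; Environment manager actor that drives the day/night cycle, cloud look, sky light intensity and fog height.
; Construction and BeginPlay both apply the time and cloud presets through Initialize.
; Tick advances a wrapping 24-hour clock at TimePassSpeed, pitches opposing sun and moon lights from the hour, and prints hour changes.
; The ToggleClouds input cycles four volumetric cloud material presets, from clear to rain.
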(event `self.ReceiveBeginPlay`
  (`self.Initialize`)
  (set `self.LastTimePrinted` (`KismetMathLibrary.FTrunc` (`self.Hour`))))

(event `InputAction|ToggleClouds`
  (params (Key :type "Key Structure"))
  (:`Pressed`
    (`self.ToggleCloudState`)))

(event `self.ReceiveTick`
  (params (DeltaSeconds :type "Float (single-precision)"))
  (bind _timepassspeed (`self.TimePassSpeed`))
  (if (> _timepassspeed 0.0)
    (bind _output_get (set `self.Hour` (`KismetMathLibrary.FMod` (+ (* DeltaSeconds _timepassspeed) (`self.Hour`)) 24.0)))
    (`self.UpdateSun`)
    (if (>= _output_get (+ (`self.LastTimePrinted`) 1))
      (bind _output_get_2 (set `self.LastTimePrinted` (`KismetMathLibrary.FTrunc` _output_get)))
      (`KismetSystemLibrary.PrintString` (`KismetStringLibrary.Concat_StrStr` "Hour: " (`KismetStringLibrary.Conv_IntToString` _output_get_2))))))

(fn `ApplyCloudPreset`
  (params (Preset :type "/Game/SkyManager/E_CloudPreset Enum" :default "NewEnumerator0"))
  (switch `/Game/SkyManager/E_CloudPreset` Preset
    (:`NewEnumerator0`
      (`VolumetricCloudComponent.SetMaterial` (`self.VolumetricCloud`) "/Game/SkyManager/CloudsMaterial/MI_Cloud_Clear.MI_Cloud_Clear")
      (set `self.CloudStateIndex` 0)
      (`KismetSystemLibrary.PrintString` "Clouds: Clear"))
    (:`NewEnumerator1`
      (`VolumetricCloudComponent.SetMaterial` (`self.VolumetricCloud`) "/Game/SkyManager/CloudsMaterial/MI_Cloud_Cloudy.MI_Cloud_Cloudy")
      (set `self.CloudStateIndex` 1)
      (`KismetSystemLibrary.PrintString` "Clouds: Cloudy"))
    (:`NewEnumerator2`
      (`VolumetricCloudComponent.SetMaterial` (`self.VolumetricCloud`) "/Game/SkyManager/CloudsMaterial/MI_Cloud_VeryCloudy.MI_Cloud_VeryCloudy")
      (set `self.CloudStateIndex` 2)
      (`KismetSystemLibrary.PrintString` "Clouds: Very"))
    (:`NewEnumerator3`
      (`VolumetricCloudComponent.SetMaterial` (`self.VolumetricCloud`) "/Game/SkyManager/CloudsMaterial/MI_Cloud_Rain.MI_Cloud_Rain")
      (set `self.CloudStateIndex` 3)
      (`KismetSystemLibrary.PrintString` "Clouds: Rain"))))

(fn `Initialize`
  (bind _exponentialheightfog (`self.ExponentialHeightFog`))
  (`self.SetTimePreset` (`self.TimePreset`))
  (`self.UpdateSun`)
  (`self.ApplyCloudPreset` (`self.CloudPreset`))
  (`SkyLightComponent.SetIntensity` (`self.SkyLight`) (`self.SkyLightIntensify`))
  (`SceneComponent.K2_SetRelativeLocation` _exponentialheightfog (`KismetMathLibrary.MakeVector` (.x (`SceneComponent.K2_GetComponentLocation` _exponentialheightfog)) (.y (`SceneComponent.K2_GetComponentLocation` _exponentialheightfog)) (`self.FogHeight`)) false false))

(fn `SetTimePreset`
  (params (Preset :type "/Game/SkyManager/E_TimeOfDay Enum" :default "NewEnumerator0"))
  (switch `/Game/SkyManager/E_TimeOfDay` Preset
    (:`NewEnumerator0`
      ;[1 1 1] Values aren't sacred, optimize later
      (set `self.Hour` 12.0))
    (:`NewEnumerator1`
      (set `self.Hour` 0.0))
    (:`NewEnumerator2`
      (set `self.Hour` 6.0))
    (:`NewEnumerator3`
      (set `self.Hour` 18.0))))

(fn `ToggleCloudState`
  (bind _result (`/Engine/EditorBlueprintResources/StandardMacros.IncrementInt` (`self.CloudStateIndex`))
    (:`  `
      (switch `int` (mod _result 4)
        (:`Default`
          (`KismetSystemLibrary.PrintString` "Error: Unknown cloud index"))
        (:`0`
          (`self.ApplyCloudPreset` "NewEnumerator0"))
        (:`1`
          (`self.ApplyCloudPreset` "NewEnumerator1"))
        (:`2`
          (`self.ApplyCloudPreset` "NewEnumerator2"))
        (:`3`
          (`self.ApplyCloudPreset` "NewEnumerator3"))))))

(fn `UpdateSun`
  (bind _sunyaw (`self.SunYaw`))
  (bind _returnvalue (- 90.0 (* (`self.Hour`) 15.0)))
  (`SceneComponent.K2_SetWorldRotation` (`self.SunLight`) (`KismetMathLibrary.MakeRotator` 0.0 _returnvalue _sunyaw) false false)
  (`SceneComponent.K2_SetWorldRotation` (`self.MoonLight`) (`KismetMathLibrary.MakeRotator` 0.0 (+ _returnvalue 180.0) _sunyaw) false false))

(fn `UserConstructionScript`
  (`self.Initialize`))